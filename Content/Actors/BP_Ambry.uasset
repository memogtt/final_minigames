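; BP_Ambry is an interactable two-door cupboard that presents an item pickup when used.
; Sphere overlaps show or hide a HUD prompt for the ThirdPersonCharacter while it is closed.
; Interact calls OpenChest, whose timeline swings the doors only if HasKey is set.
; Regardless of key, it then zooms the camera, opens the item screen with mouse input and spawns ItemClassSpawn above the chest, applying Mesh to the pickup.
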(event OnComponentBeginOverlap(Sphere)
  (params (OverlappedComponent :type Primitive%20Component%20Object%20Reference) (OtherActor :type Actor%20Object%20Reference) (OtherComp :type Primitive%20Component%20Object%20Reference) (OtherBodyIndex :type Integer) (bFromSweep :type Boolean) (SweepResult :type Hit%20Result%20Structure%20%28by%20ref%29))
  (if (not (Variables|Default|GetisOpen))
    (bind _asthird_person_character (Utilities|Casting|CastToThirdPersonCharacter OtherActor))
    (Default|ShowTextFade (Variables|/Game/ThirdPersonBP/Blueprints/ThirdPersonCharacter.ThirdPersonCharacter_C|GetHUD _asthird_person_character) (Variables|Default|GetText))))

(event OnComponentEndOverlap(Sphere)
  (params (OverlappedComponent :type Primitive%20Component%20Object%20Reference) (OtherActor :type Actor%20Object%20Reference) (OtherComp :type Primitive%20Component%20Object%20Reference) (OtherBodyIndex :type Integer))
  (if (not (Variables|Default|GetisOpen))
    (bind _asthird_person_character (Utilities|Casting|CastToThirdPersonCharacter OtherActor))
    (Default|HideTextFade (Variables|/Game/ThirdPersonBP/Blueprints/ThirdPersonCharacter.ThirdPersonCharacter_C|GetHUD _asthird_person_character))))

(event Custom|OpenChest
  (if (Variables|Default|GetHasKey)
    (Variables|Default|SetisOpen true)
    (Audio|PlaySoundatLocation "/Game/sound/puertitas.puertitas" (Variables|/Script/Engine.SceneComponent|GetRelativeLocation (Variables|Default|Getchest)) "0, 0, 0" 1.0 1.0 0.0 0 0 0)
    (bind _newtrack_0 (Timeline|Timeline_0 Play)
      (:Update
        (Transformation|SetRelativeRotation (Variables|Default|Getdoor1) (Math|Rotator|Lerp(Rotator) "0,-90.000000, 0" "0, 0, 0" _newtrack_0) false false)
        (Transformation|SetRelativeRotation (Variables|Default|Getdoor2) (Math|Rotator|Lerp(Rotator) "0.000000,-270.000000,180.000000" "0,-360.000000,180.000000" _newtrack_0) false false)))))

(event Custom|CloseChest
  (Variables|Default|SetisOpen false)
  (bind _newtrack_0 (Timeline|Timeline_0 Reverse)
    (:Update
      (Transformation|SetRelativeRotation (Variables|Default|Getdoor1) (Math|Rotator|Lerp(Rotator) "0,-90.000000, 0" "0, 0, 0" _newtrack_0) false false)
      (Transformation|SetRelativeRotation (Variables|Default|Getdoor2) (Math|Rotator|Lerp(Rotator) "0.000000,-270.000000,180.000000" "0,-360.000000,180.000000" _newtrack_0) false false))))

(event EventBeginPlay)

(event Collision|EventActorBeginOverlap
  (params (OtherActor :type Actor%20Object%20Reference)))

(event EventInteract
  (params (instigator :type Actor%20Object%20Reference))
  (bind _returnvalue (Game|GetPlayerController 0))
  (bind _chest (Variables|Default|Getchest))
  (bind _returnvalue_2 (Transformation|GetSocketTransform _chest "None" "RTS_World"))
  (bind (_location _rotation _scale) (Math|Transform|BreakTransform _returnvalue_2))
  (bind (_x _y _z) (Math|Vector|BreakVector _location))
  (if (not (Variables|Default|GetisOpen))
    (CallFunction|OpenChest)
    (bind _asthird_person_character (Utilities|Casting|CastToThirdPersonCharacter instigator))
    (Default|HideTextFade (Variables|/Game/ThirdPersonBP/Blueprints/ThirdPersonCharacter.ThirdPersonCharacter_C|GetHUD _asthird_person_character))
    (Utilities|FlowControl|Delay 0.8)
    (Default|CameraZoomin _asthird_person_character)
    (bind _returnvalue_3 (UserInterface|CreateWidget "/Game/Widgets/WB_ItemScreen.WB_ItemScreen_C"))
    (bind _output_get (Variables|/Game/ThirdPersonBP/Blueprints/ThirdPersonCharacter.ThirdPersonCharacter_C|SetItemHUD _asthird_person_character _returnvalue_3))
    (UserInterface|Viewport|AddtoViewport _output_get 0)
    (Variables|/Script/Engine.PlayerController|SetbShowMouseCursor _returnvalue true)
    (Input|SetInputModeGameandUI _returnvalue 0 "DoNotLock" true)
    (bind _returnvalue_4 (Game|SpawnActorfromClass (Variables|Default|GetItemClassSpawn) (Math|Transform|MakeTransform (Math|Vector|MakeVector _x _y (+ _z 4e+01)) _rotation _scale) "Undefined" 0 0))
    (bind _asbp_pickup (Utilities|Casting|CastToBP_Pickup _returnvalue_4))
    (Components|StaticMesh|SetStaticMesh (Variables|/Game/Actors/BP_Pickup.BP_Pickup_C|Getobject _asbp_pickup) (Variables|Default|Getmesh))))

(fn ConstructionScript)