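; Alchemist table actor where the player places five found potions and, once all are placed, opens a potion crafting widget.
; A box overlap shows or hides a HUD prompt that depends on CanCraft.
; Interact reveals a potion mesh for each one the character holds and sets CanCraft from the character's PotionsComplete check.
; When CanCraft is true, Interact instead creates WB_Potions and enables the mouse cursor with Game and UI input.
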(event OnComponentBeginOverlap(Box)
  (params (OverlappedComponent :type Primitive%20Component%20Object%20Reference) (OtherActor :type Actor%20Object%20Reference) (OtherComp :type Primitive%20Component%20Object%20Reference) (OtherBodyIndex :type Integer) (bFromSweep :type Boolean) (SweepResult :type Hit%20Result%20Structure%20%28by%20ref%29))
  (bind _asthird_person_character (Utilities|Casting|CastToThirdPersonCharacter OtherActor))
  (if (Variables|Default|GetcanCraft)
    (Default|ShowTextFade (Variables|/Game/ThirdPersonBP/Blueprints/ThirdPersonCharacter.ThirdPersonCharacter_C|GetHUD _asthird_person_character) "Press E to craft")
    (else
      (Default|ShowTextFade (Variables|/Game/ThirdPersonBP/Blueprints/ThirdPersonCharacter.ThirdPersonCharacter_C|GetHUD _asthird_person_character) "Place potions, you need to find 5!!"))))

(event OnComponentEndOverlap(Box)
  (params (OverlappedComponent :type Primitive%20Component%20Object%20Reference) (OtherActor :type Actor%20Object%20Reference) (OtherComp :type Primitive%20Component%20Object%20Reference) (OtherBodyIndex :type Integer))
  (bind _asthird_person_character (Utilities|Casting|CastToThirdPersonCharacter OtherActor))
  (Default|HideTextFade (Variables|/Game/ThirdPersonBP/Blueprints/ThirdPersonCharacter.ThirdPersonCharacter_C|GetHUD _asthird_person_character)))

(event EventBeginPlay)

(event Collision|EventActorBeginOverlap
  (params (OtherActor :type Actor%20Object%20Reference)))

(event EventTick
  (params (DeltaSeconds :type Float%20%28single-precision%29)))

(event EventInteract
  (params (instigator :type Actor%20Object%20Reference))
  (bind _returnvalue (Game|GetPlayerController 0))
  (if (Variables|Default|GetcanCraft)
    (Default|HideTextFade (Variables|/Game/ThirdPersonBP/Blueprints/ThirdPersonCharacter.ThirdPersonCharacter_C|GetHUD (stale _asthird_person_character)))
    (Variables|/Script/Engine.PlayerController|SetbShowMouseCursor _returnvalue true)
    (Input|SetInputModeGameandUI _returnvalue 0 "DoNotLock" true)
    (bind _returnvalue_2 (UserInterface|CreateWidget "/Game/Widgets/WB_Potions.WB_Potions_C"))
    (UserInterface|Viewport|AddtoViewport _returnvalue_2 0)
    (else
      (bind _asthird_person_character (Utilities|Casting|CastToThirdPersonCharacter instigator))
      (for (_array_element _array_index) (Variables|/Game/ThirdPersonBP/Blueprints/ThirdPersonCharacter.ThirdPersonCharacter_C|Getpotions _asthird_person_character)
        (switch int _array_index
          (:0
            (if _array_element
              (Rendering|SetVisibility (Variables|Default|Getpotion1) true false)
              (bind _complete (Default|PotionsComplete _asthird_person_character :!label _label))
              (bind _output_get (Variables|Default|SetcanCraft _complete))
              (if _output_get
                (Default|ShowTextFade (Variables|/Game/ThirdPersonBP/Blueprints/ThirdPersonCharacter.ThirdPersonCharacter_C|GetHUD _asthird_person_character) "Press E to craft"))))
          (:1
            (if _array_element
              (Rendering|SetVisibility (Variables|Default|Getpotion2) true false)
              (goto _label)))
          (:2
            (if _array_element
              (Rendering|SetVisibility (Variables|Default|Getpotion3) true false)
              (goto _label)))
          (:3
            (if _array_element
              (Rendering|SetVisibility (Variables|Default|Getpotion4) true false)
              (goto _label)))
          (:4
            (if _array_element
              (Rendering|SetVisibility (Variables|Default|Getpotion5) true false)
              (goto _label))))))))

(fn ConstructionScript)