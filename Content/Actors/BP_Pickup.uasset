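; BP_Pickup is an interactable pickup whose static mesh is set from its Mesh variable in the construction script.
; On Interact, it zooms out the third-person character's ItemHUD, flags any potion in that character's Potions array, plays a sound and destroys itself.
; PotionNum derives the potion index by parsing the single digit after "Potion_" in the mesh's asset path, so mesh naming determines the potion granted.
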(event EventBeginPlay)

(event Collision|EventActorBeginOverlap
  (params (OtherActor :type Actor%20Object%20Reference)))

(event EventTick
  (params (DeltaSeconds :type Float%20%28single-precision%29)))

(event EventInteract
  (params (instigator :type Actor%20Object%20Reference))
  (bind _asthird_person_character (Utilities|Casting|CastToThirdPersonCharacter instigator))
  (Utilities|IsValid (Variables|/Game/ThirdPersonBP/Blueprints/ThirdPersonCharacter.ThirdPersonCharacter_C|GetItemHUD _asthird_person_character)
    (:Is%20Valid
      (Default|ZoomOut (Variables|/Game/ThirdPersonBP/Blueprints/ThirdPersonCharacter.ThirdPersonCharacter_C|GetItemHUD _asthird_person_character)))
    (:Is%20Not%20Valid
      _))
  (bind _potion (CallFunction|PotionNum))
  (if (>= _potion 0)
    (Utilities|Array|SetArrayElem (Variables|/Game/ThirdPersonBP/Blueprints/ThirdPersonCharacter.ThirdPersonCharacter_C|Getpotions _asthird_person_character) _potion true))
  (Audio|PlaySoundatLocation "/Game/sound/pickup.pickup" (Variables|/Script/Engine.SceneComponent|GetRelativeLocation (Variables|Default|Getobject)) "0, 0, 0" 1.0 1.0 0.0 0 0 0)
  (Actor|DestroyActor))

(fn ConstructionScript
  (Components|StaticMesh|SetStaticMesh (Variables|Default|Getobject) (Variables|Default|Getmesh)))

(fn PotionNum
  (bind _mesh (Variables|Default|Getmesh))
  (bind _returnvalue (Class|KismetSystemLibrary|GetPathName _mesh))
  (bind _returnvalue_2 (Utilities|String|FindSubstring _returnvalue "Potion_"))
  (if (> _returnvalue_2 0)
    (return (- (Math|Conversions|ToInteger(Byte) (Utilities|String|GetSubstring _returnvalue (+ _returnvalue_2 7))) 1))
    (else
      (return -1))))