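; BP_Read is an interactable readable actor that shows its text in a scroll widget.
; At BeginPlay it applies its Mesh variable to the StaticMesh component.
; On Interact it creates a WB_Scroll, passes NewText to ShowTextFade, adds it to the viewport, then switches player 0 to Game and UI input with a visible cursor.
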(event EventBeginPlay
  (Components|StaticMesh|SetStaticMesh (Variables|Default|GetStaticMesh) (Variables|Default|Getmesh)))

(event Collision|EventActorBeginOverlap
  (params (OtherActor :type Actor%20Object%20Reference)))

(event EventTick
  (params (DeltaSeconds :type Float%20%28single-precision%29)))

(event EventInteract
  (params (instigator :type Actor%20Object%20Reference))
  (bind _returnvalue (Game|GetPlayerController 0))
  (bind _returnvalue_2 (UserInterface|CreateWidget "/Game/Widgets/WB_Scroll.WB_Scroll_C"))
  (Default|ShowTextFade _returnvalue_2 (Variables|Default|GetNewText))
  (UserInterface|Viewport|AddtoViewport _returnvalue_2 0)
  (Input|SetInputModeGameandUI _returnvalue 0 "DoNotLock" true)
  (Variables|/Script/Engine.PlayerController|SetbShowMouseCursor _returnvalue true))

(fn ConstructionScript)