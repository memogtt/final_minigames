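; BP_bookshelf is an interactable bookshelf that slides aside once, when a character with strength moves it.
; On Interact it casts the instigator to ThirdPersonCharacter and checks HasStrength, otherwise prompting a dialog that the player is too weak.
; On success it sets IsOpen, plays a sound, and a timeline lerps the static mesh's relative location sideways along X.
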(event EventBeginPlay)

(event Collision|EventActorBeginOverlap
  (params (OtherActor :type Actor%20Object%20Reference)))

(event EventTick
  (params (DeltaSeconds :type Float%20%28single-precision%29)))

(event EventInteract
  (params (instigator :type Actor%20Object%20Reference))
  (if (not (Variables|Default|GetIsOpen))
    (bind _asthird_person_character (Utilities|Casting|CastToThirdPersonCharacter instigator))
    (if (Variables|/Game/ThirdPersonBP/Blueprints/ThirdPersonCharacter.ThirdPersonCharacter_C|GethasStrength _asthird_person_character)
      (Variables|Default|SetisOpen true)
      (Audio|PlaySoundatLocation "/Game/sound/puertitas.puertitas" (Variables|/Script/Engine.SceneComponent|GetRelativeLocation (Variables|Default|GetStaticMesh)) "0, 0, 0" 1.0 1.0 0.0 0 0 0)
      (bind _newtrack_0 (Timeline|Timeline_0 Play)
        (:Update
          (Transformation|SetRelativeLocation (Variables|Default|GetStaticMesh) (Math|Vector|Lerp(Vector) "0, 0, 0" "-120.000000, 0, 0" _newtrack_0) false false)))
      (else
        (Default|PromptDialog _asthird_person_character " It seems you are not STRONG enough to move it")))))

(fn ConstructionScript)