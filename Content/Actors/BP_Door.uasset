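; BP_Door is a double door that swings open when the ThirdPersonCharacter comes near, provided its HasKey flag is true.
; Sphere overlap events call OpenDoor on entry and CloseDoor after a short delay on exit.
; A single Timeline drives rotation lerps that swing the Left and Right components in opposite directions, playing forward to open and reversing to close.
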(event OnComponentBeginOverlap(Sphere)
  (params (OverlappedComponent :type Primitive%20Component%20Object%20Reference) (OtherActor :type Actor%20Object%20Reference) (OtherComp :type Primitive%20Component%20Object%20Reference) (OtherBodyIndex :type Integer) (bFromSweep :type Boolean) (SweepResult :type Hit%20Result%20Structure%20%28by%20ref%29))
  (Utilities|Casting|CastToThirdPersonCharacter OtherActor)
  (CallFunction|OpenDoor))

(event OnComponentEndOverlap(Sphere)
  (params (OverlappedComponent :type Primitive%20Component%20Object%20Reference) (OtherActor :type Actor%20Object%20Reference) (OtherComp :type Primitive%20Component%20Object%20Reference) (OtherBodyIndex :type Integer))
  (Utilities|Casting|CastToThirdPersonCharacter OtherActor)
  (Utilities|FlowControl|Delay 1.0)
  (CallFunction|CloseDoor))

(event Custom|OpenDoor
  (if (Variables|Default|GetHasKey)
    (bind _newtrack_0 (Timeline|Timeline_0 Play)
      (:Update
        (Transformation|SetRelativeRotation (Variables|Default|Getright) (Math|Rotator|Lerp(Rotator) "0, 0, 0" "0.000000,90.000000,0.000000" _newtrack_0) false false)
        (Transformation|SetRelativeRotation (Variables|Default|Getleft) (Math|Rotator|Lerp(Rotator) "0,180.000000, 0" "0.000000,90.000000,0.000000" _newtrack_0) false false)))))

(event Custom|CloseDoor
  (bind _newtrack_0 (Timeline|Timeline_0 Reverse)
    (:Update
      (Transformation|SetRelativeRotation (Variables|Default|Getright) (Math|Rotator|Lerp(Rotator) "0, 0, 0" "0.000000,90.000000,0.000000" _newtrack_0) false false)
      (Transformation|SetRelativeRotation (Variables|Default|Getleft) (Math|Rotator|Lerp(Rotator) "0,180.000000, 0" "0.000000,90.000000,0.000000" _newtrack_0) false false))))

(event EventBeginPlay)

(event Collision|EventActorBeginOverlap
  (params (OtherActor :type Actor%20Object%20Reference)))

(event EventTick
  (params (DeltaSeconds :type Float%20%28single-precision%29)))

(fn ConstructionScript)